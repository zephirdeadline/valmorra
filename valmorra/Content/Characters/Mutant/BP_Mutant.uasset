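; BP_Mutant is a Mutant character Blueprint that adds a death animation to behavior inherited from its parent class.
; Its Dying event calls the parent implementation, then plays the non-looping Mutant_Dying animation directly on the mesh.
; BeginPlay, overlap and Tick are disabled placeholder nodes, and the construction script only calls the parent.
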(event `self.Dying`
  (params (`luck%` :type "Float (double-precision)"))
  (`parent.Dying` 0.0)
  (`SkeletalMeshComponent.PlayAnimation` (`self.Mesh`) "/Game/Characters/Mutant/Mutant_Dying.Mutant_Dying" false))

(fn `UserConstructionScript`
  (`parent.UserConstructionScript`))