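; BP_Mob is a mob character with stats, a life bar widget and random loot drops on death.
; GetDamage subtracts the CalcDamages result of attacker versus mob stats from life, then refreshes the widget against MaxLife.
; At zero life, Dying disables collision and rolls each loot entry's probability plus Luck (passed as zero here).
; Successful rolls spawn loot actors scattered near the capsule's base, and a timer later destroys the mob.
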(event `self.ReceiveBeginPlay`
  (bind _stats_life (break `/Game/Content/Structures/S_Stats` (`self.stats`)))
  (set `self.MaxLife` _stats_life)
  (`self.Update_UI_stat`))

(event `Dying`
  (params (`luck%` :type "Float (double-precision)"))
  (bind _capsulecomponent (`self.CapsuleComponent`))
  (bind (_returnvalue_x _returnvalue_y _returnvalue_z) (`KismetMathLibrary.BreakVector` (`SceneComponent.K2_GetComponentLocation` _capsulecomponent)))
  (`self.SetActorEnableCollision` false)
  (for _array_element (`self.Loots`)
    (if (<= (`KismetMathLibrary.RandomFloat`) (/ (+ (`.Probability_14_E36D615A419ED90EADFC1CAF73C5A9C9` (break `/Game/Content/Structures/Loot` _array_element)) `luck%`) 100.0))
      (`|SpawnActorFromClass` :`Class` "/Game/Content/Loot.Loot_C" :`SpawnTransform` (`KismetMathLibrary.MakeTransform` (`KismetMathLibrary.MakeVector` (+ (`KismetMathLibrary.RandomFloatInRange` -200.0 200.0) _returnvalue_x) (+ _returnvalue_y (`KismetMathLibrary.RandomFloatInRange` -200.0 200.0)) (- _returnvalue_z (+ (`.OutHalfHeight` (`CapsuleComponent.GetScaledCapsuleSize` _capsulecomponent)) -20.0)))) :`CollisionHandlingOverride` "Undefined" :`TransformScaleMethod` "MultiplyWithRoot" :`Loots` (`|MakeArray` _array_element) :`Instigator` null)))
  (`KismetSystemLibrary.K2_SetTimerDelegate` (delegate `Dispawn`) 20.0))

(event `Dispawn`
  (`self.K2_DestroyActor`))

(event `GetDamage`
  (params (TotalStatsHiter :type "/Game/Content/Structures/S_Stats Structure") (ActorHiter :type "Actor Object Reference"))
  (bind _stats_life (break `/Game/Content/Structures/S_Stats` (`self.stats`)))
  (bind _stats_life_2 (break `/Game/Content/Structures/S_Stats` (`self.stats`)))
  (bind _damages (`/Game/Content/LibGlobale.CalcDamages` TotalStatsHiter (`self.stats`)))
  (setmembers `/Game/Content/Structures/S_Stats` :`StructRef` (`self.stats`) :`life` (- _stats_life_2 _damages))
  (if (<= _stats_life 0)
    (`self.Dying` 0.0))
  (`self.Update_UI_stat`))

(event `Update_UI_stat`
  (bind _stats_life (break `/Game/Content/Structures/S_Stats` (`self.stats`)))
  (bind _stats_life_2 (break `/Game/Content/Structures/S_Stats` (`self.stats`)))
  (bind _asui_mob_stat (cast `/Game/Content/UI/UI_Mob_Stat` (`WidgetComponent.GetWidget` (`self.Widget`)) :!pure true))
  (set `ProgressBar.Percent` (/ _stats_life (`self.MaxLife`)) (`/Game/Content/UI/UI_Mob_Stat.ProgressBar_Life` _asui_mob_stat))
  (`TextBlock.SetText` (`/Game/Content/UI/UI_Mob_Stat.Total_Life` _asui_mob_stat) (`KismetTextLibrary.Conv_StringToText` (`KismetStringLibrary.Concat_StrStr` (`KismetStringLibrary.Conv_IntToString` _stats_life_2) "/" (`KismetStringLibrary.Conv_IntToString` (`self.MaxLife`))))))

(fn `UserConstructionScript`
  (bind _stats_life (break `/Game/Content/Structures/S_Stats` (`self.stats`)))
  (set `self.MaxLife` _stats_life))