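; BP_Interactive is an interactive actor Blueprint that carries a widget listing its available actions.
; ShowAction and HideAction toggle the WidgetActions component, while AddInput appends a UI_ItemAction entry with shortcut and description to the UI_Action_Item list.
; Empty F, R and T events act as action hooks, with only R receiving a Player.
; BeginPlay, overlap and Tick are unused, so nothing here triggers the display itself.
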(event `ShowAction`
  (`SceneComponent.SetVisibility` (`self.Widget_actions`) true false))

(event `HideAction`
  (`SceneComponent.SetVisibility` (`self.Widget_actions`) false false))

(event `Add Input`
  (params (shortcut :type Text) (Desc :type Text))
  (bind _asui_action_item (cast `/Game/Content/UI/UI_Action_Item` (`WidgetComponent.GetWidget` (`self.Widget_actions`))))
  (bind _returnvalue (`|CreateWidget` "/Game/Content/UI/UI_ItemAction.UI_ItemAction_C" null shortcut Desc))
  (`VerticalBox.AddChildToVerticalBox` (`/Game/Content/UI/UI_Action_Item.Actions_list` _asui_action_item) _returnvalue))

(event `F`)

(event `R`
  (params (player :type "/Game/ThirdPerson/Blueprints/BP_ThirdPersonCharacter Object Reference")))

(event `T`)

(fn `UserConstructionScript`)