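; Lootable chest that registers an R "Loot" action through inherited interaction logic.
; On R it passes each item in Loots to the player's CPInventory, prints debug text, calls MultiR to open the chest, then empties the array.
; The OpenChest timeline pitches an arrow component to open, and reverses to close when the action prompt is hidden.
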(event `self.ReceiveBeginPlay`
  (`self.Add Input` "R" "Loot"))

(event `Open`
  (bind (_direction _angle) (`Timeline|Open Chest` :!label _label)
    (:`Update`
      (`SceneComponent.K2_SetRelativeRotation` (`self.Arrow_0`) (`KismetMathLibrary.MakeRotator` 0.0 _angle) false false))))

(event `Close`
  (goto _label :!via `Reverse`))

(event `self.ShowAction`
  (`parent.ShowAction`))

(event `self.HideAction`
  (`parent.HideAction`)
  (`self.Close`))

(event `self.R`
  (params (player :type "/Game/ThirdPerson/Blueprints/BP_ThirdPersonCharacter Object Reference"))
  (bind _loots (`self.loots`))
  (`KismetSystemLibrary.PrintText` (`KismetTextLibrary.Conv_IntToText` (`KismetArrayLibrary.Array_Length` _loots)))
  (for (_array_element _array_index) _loots
    (`KismetSystemLibrary.PrintText` (`KismetTextLibrary.Conv_NameToText` (`.ItemID_6_704D7B7E45F191F293DA24A87B67714A` (break `/Game/Content/Structures/Loot` _array_element))))
    (`/Game/Content/CP_Inventory.Add Item` (`/Game/ThirdPerson/Blueprints/BP_ThirdPersonCharacter.CP_Inventory` player) _array_element))
  (`self.Multi R`)
  (`KismetArrayLibrary.Array_Clear` _loots))

(event `Multi R`
  (`self.Open`))

(fn `UserConstructionScript`)